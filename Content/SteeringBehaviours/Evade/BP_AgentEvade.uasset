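; BP_AgentEvade is a steering-behaviour agent that evades the BP_Target actor found at BeginPlay.
; Each Tick, Evade passes Flee a predicted point, though target velocity is fixed at zero, so it is just the target's location tripled.
; Flee negates the seek steering force, sets the Cone's physics velocity at constant MaxVel and has optional debug drawing.
; LookAtDirection then orients the Cone from that velocity, zeroing pitch.
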(event EventBeginPlay
  (bind _output_get (Variables|Default|SetCurrentVel "0, 0, 0"))
  (Physics|SetPhysicsLinearVelocity (Variables|Default|GetCone) (* (Math|Vector|Normalize _output_get) (Variables|Default|GetMaxVel)) false "None")
  (bind _returnvalue (Actor|GetActorOfClass "/Game/SteeringBehaviours/Seek/BP_Target.BP_Target_C"))
  (Variables|Default|SetTarget _returnvalue))

(event EventTick
  (params (DeltaSeconds :type Float%20%28single-precision%29))
  ;[0.9952 0.6059 1] Flee
  (CallFunction|Evade (Transformation|GetWorldLocation (Variables|/Script/Engine.Actor|GetRootComponent (Variables|Default|GetTarget))))
  ;[1 0.5831 0.6734] Rotation
  (CallFunction|LookatDirection))

(fn ConstructionScript)

(fn Flee
  (params (Pos :type Vector) (Debug :type Boolean))
  (bind _cone (Variables|Default|GetCone))
  (bind _cone_2 (Variables|Default|GetCone))
  (bind _relativelocation (Variables|/Script/Engine.SceneComponent|GetRelativeLocation _cone))
  (bind _relativelocation_2 (Variables|/Script/Engine.SceneComponent|GetRelativeLocation _cone_2))
  (LocalVariables|SetTargetPos Pos)
  (LocalVariables|Set_Debug Debug)
  (Utilities|FlowControl|Sequence
    (:then_0
      ;[0.9985 0.5077 1] Create Desired Vel
      (Variables|Default|SetDesiredVel (* (Math|Vector|Normalize (- (LocalVariables|GetTargetPos) (Variables|/Script/Engine.SceneComponent|GetRelativeLocation (Variables|Default|GetCone)))) (Variables|Default|GetMaxVel))))
    (:then_1
      ;[0.4883 0.4619 1] Desired Vel
      (if (LocalVariables|Get_Debug)
        (Rendering|Debug|DrawDebugLine _relativelocation_2 (+ _relativelocation_2 (Variables|Default|GetDesiredVel)) "(R=0.000000,G=0.000000,B=0.000000,A=1.000000)" 0.0 0.0)))
    (:then_2
      ;[0.4356 1 0.6083] Steering Vel
      (Variables|Default|SetSteering (* (Math|Vector|Normalize (- (Variables|Default|GetDesiredVel) (Variables|Default|GetCurrentVel))) (Variables|Default|GetMaxForce))))
    (:then_3
      ;[0.3294 0.7767 1] Steering
      (if (LocalVariables|Get_Debug)
        (Rendering|Debug|DrawDebugArrow :LineStart (+ (Variables|/Script/Engine.SceneComponent|GetRelativeLocation (Variables|Default|GetCone)) (Variables|Default|GetCurrentVel)) :LineEnd (+ (+ (Variables|/Script/Engine.SceneComponent|GetRelativeLocation (Variables|Default|GetCone)) (Variables|Default|GetCurrentVel)) (Variables|Default|GetSteering)))))
    (:then_4
      ;[0.7037 1 0.5271] Add Steering to CurrentVel
      (Variables|Default|SetCurrentVel (* (Math|Vector|Normalize (+ (Variables|Default|GetCurrentVel) (* (Variables|Default|GetSteering) -1))) (Variables|Default|GetMaxVel))))
    (:then_5
      ;[0.6573 0.3742 1] CurrentVel
      (if (LocalVariables|Get_Debug)
        (Rendering|Debug|DrawDebugLine :LineStart _relativelocation :LineEnd (+ _relativelocation (Variables|Default|GetCurrentVel)))))
    (:then_6
      ;[1 0.3996 0.4394] Apply Force
      (Physics|SetPhysicsLinearVelocity (Variables|Default|GetCone) (Variables|Default|GetCurrentVel) false "None"))))

(fn LookatDirection
  (bind _cone (Variables|Default|GetCone))
  (bind _currentvel (Variables|Default|GetCurrentVel))
  (bind _cone_2 (Variables|Default|GetCone))
  (bind _returnvalue (Transformation|GetWorldLocation _cone_2))
  (bind _relativelocation (Variables|/Script/Engine.SceneComponent|GetRelativeLocation _cone))
  (bind _returnvalue_2 (- _relativelocation _currentvel))
  (bind _returnvalue_3 (Math|Rotator|FindLookatRotation _returnvalue _returnvalue_2))
  (bind (_roll _pitch _yaw) (Math|Rotator|BreakRotator _returnvalue_3))
  ;[0.6787 1 0.9092] Rotate
  (Transformation|SetWorldRotation (Variables|Default|GetCone) (Math|Rotator|MakeRotator _roll 0.0 _yaw) false false))

(fn Evade
  (params (Target :type Vector))
  (bind _output_get (LocalVariables|SetTargetVel "0, 0, 0"))
  (LocalVariables|SetT 3)
  (bind _output_get_2 (LocalVariables|SetPrediction (* (+ Target _output_get) (LocalVariables|GetT))))
  (CallFunction|Flee _output_get_2 false))