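; Flocking agent, apparently an unfinished boids prototype, built on a physics Cone that finds a BP_TargetF at BeginPlay but never uses it.
; Each tick, Flocking adds Alignment, Cohesion and Separation to CurrentVel, unweighted then weighted, and LookAtDirection rotates the Cone from it.
; Alignment sums nearby FollowingAgents' positions, but its averaging and part of Separation are unwired.
; Physics velocity is set only at BeginPlay, from a zero vector.
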(event EventBeginPlay
  ;[0.4042 0.6378 1] Add inicial vel
  (bind _output_get (Variables|Default|SetCurrentVel "0, 0, 0"))
  (Physics|SetPhysicsLinearVelocity (Variables|Default|GetCone) (* (Math|Vector|Normalize _output_get) (Variables|Default|GetMaxVel)) false "None")
  (bind _returnvalue (Actor|GetActorOfClass "/Game/SteeringBehaviours/Flocking/BP_TargetF.BP_TargetF_C"))
  (Variables|Default|SetTarget _returnvalue))

(event EventTick
  (params (DeltaSeconds :type Float%20%28single-precision%29))
  ;[0.9952 0.6059 1] Seek
  (CallFunction|Flocking)
  ;[1 0.5831 0.6734] Rotation
  (CallFunction|LookatDirection))

(fn ConstructionScript)

(fn LookatDirection
  (bind _cone (Variables|Default|GetCone))
  (bind _currentvel (Variables|Default|GetCurrentVel))
  (bind _cone_2 (Variables|Default|GetCone))
  (bind _returnvalue (Transformation|GetWorldLocation _cone))
  (bind _relativelocation (Variables|/Script/Engine.SceneComponent|GetRelativeLocation _cone_2))
  (bind _returnvalue_2 (- _relativelocation _currentvel))
  (bind _returnvalue_3 (Math|Rotator|FindLookatRotation _returnvalue _returnvalue_2))
  (bind (_roll _pitch _yaw) (Math|Rotator|BreakRotator _returnvalue_3))
  ;[0.6787 1 0.9092] Rotate
  (Transformation|SetWorldRotation (Variables|Default|GetCone) (Math|Rotator|MakeRotator _roll 0.0 _yaw) false false))

(fn Alignment
  (Variables|Default|SetV "0, 0, 0")
  (Variables|Default|SetNCount 0)
  (for _array_element (Variables|Default|GetFollowingAgents)
    (if (!= _array_element (Variables|Default|GetCone))
      (if (< (Math|Vector|Distance(Vector) (Transformation|GetActorLocation _array_element) (Variables|/Script/Engine.SceneComponent|GetRelativeLocation (Variables|Default|GetCone))) 3e+02)
        (Variables|Default|SetCurrentVel (Math|Conversions|ToVector(Float) (.X (Math|Vector|BreakVector (+ (.X (Math|Vector|BreakVector (Variables|Default|GetCurrentVel))) (.X (Math|Vector|BreakVector (Transformation|GetActorLocation _array_element))))))))
        (Variables|Default|SetCurrentVel (Math|Conversions|ToVector(Float) (.Y (Math|Vector|BreakVector (Math|Conversions|ToVector(Float) (+ (.Y (Math|Vector|BreakVector (Variables|Default|GetCurrentVel))) (.Y (Math|Vector|BreakVector (Transformation|GetActorLocation _array_element)))))))))
        (Variables|Default|SetCurrentVel (Math|Conversions|ToVector(Float) (.Z (Math|Vector|BreakVector (Math|Conversions|ToVector(Float) (+ (.Z (Math|Vector|BreakVector (Variables|Default|GetCurrentVel))) (.Z (Math|Vector|BreakVector (Transformation|GetActorLocation _array_element)))))))))
        (Variables|Default|SetNCount (+ 1 (Variables|Default|GetNCount)))))))

(fn Cohesion
  (Variables|Default|SetV (Math|Conversions|ToVector(Float) (+ (.X (Math|Vector|BreakVector (Variables|Default|GetV))) (.X (Math|Vector|BreakVector (Variables|/Script/Engine.SceneComponent|GetRelativeLocation (Variables|Default|GetCone)))))))
  (Variables|Default|SetV (Math|Conversions|ToVector(Float) (+ (.Y (Math|Vector|BreakVector (Variables|Default|GetV))) (.Y (Math|Vector|BreakVector (Variables|/Script/Engine.SceneComponent|GetRelativeLocation (Variables|Default|GetCone)))))))
  (Variables|Default|SetV (Math|Conversions|ToVector(Float) (+ (.Z (Math|Vector|BreakVector (Variables|Default|GetV))) (.Z (Math|Vector|BreakVector (Variables|/Script/Engine.SceneComponent|GetRelativeLocation (Variables|Default|GetCone)))))))
  (Variables|Default|SetV (Math|Conversions|ToVector(Float) (/ (.X (Math|Vector|BreakVector (Variables|Default|GetV))) (Variables|Default|GetNCount))))
  (Variables|Default|SetV (Math|Conversions|ToVector(Float) (/ (.Y (Math|Vector|BreakVector (Variables|Default|GetV))) (Variables|Default|GetNCount))))
  (Variables|Default|SetV (Math|Conversions|ToVector(Float) (/ (.Z (Math|Vector|BreakVector (Variables|Default|GetV))) (Variables|Default|GetNCount))))
  (Variables|Default|SetV (Math|Conversions|ToVector(Float) (- (.X (Math|Vector|BreakVector (Variables|Default|GetV))) (.X (Math|Vector|BreakVector (Variables|/Script/Engine.SceneComponent|GetRelativeLocation (Variables|Default|GetCone)))))))
  (Variables|Default|SetV (Math|Conversions|ToVector(Float) (- (.Y (Math|Vector|BreakVector (Variables|Default|GetV))) (.Y (Math|Vector|BreakVector (Variables|/Script/Engine.SceneComponent|GetRelativeLocation (Variables|Default|GetCone)))))))
  (bind _output_get (Variables|Default|SetV (Math|Conversions|ToVector(Float) (- (.Z (Math|Vector|BreakVector (Variables|Default|GetV))) (.Z (Math|Vector|BreakVector (Variables|/Script/Engine.SceneComponent|GetRelativeLocation (Variables|Default|GetCone))))))))
  (return (Math|Vector|Normalize _output_get 1.0)))

(fn Separation
  (Variables|Default|SetV (Math|Conversions|ToVector(Float) (- (.X (Math|Vector|BreakVector (Variables|Default|GetV))) (.X (Math|Vector|BreakVector (Variables|/Script/Engine.SceneComponent|GetRelativeLocation (Variables|Default|GetCone)))))))
  (Variables|Default|SetV (Math|Conversions|ToVector(Float) (- (.Y (Math|Vector|BreakVector (Variables|Default|GetV))) (.Y (Math|Vector|BreakVector (Variables|/Script/Engine.SceneComponent|GetRelativeLocation (Variables|Default|GetCone)))))))
  (Variables|Default|SetV (Math|Conversions|ToVector(Float) (- (.Z (Math|Vector|BreakVector (Variables|Default|GetV))) (.Z (Math|Vector|BreakVector (Variables|/Script/Engine.SceneComponent|GetRelativeLocation (Variables|Default|GetCone))))))))

(fn Flocking
  (Utilities|FlowControl|Sequence
    (:then_0
      (bind _vel (CallFunction|Alignment))
      (LocalVariables|Setaligment _vel))
    (:then_1
      (bind _v (CallFunction|Cohesion))
      (LocalVariables|Setcohesion _v))
    (:then_2
      (bind _v_2 (CallFunction|Separation))
      (LocalVariables|Setseparation _v_2))
    (:then_3
      (Variables|Default|SetCurrentVel (+ (.X (Math|Vector|BreakVector (Variables|Default|GetCurrentVel))) (+ (.X (Math|Vector|BreakVector (LocalVariables|Getaligment))) (.X (Math|Vector|BreakVector (LocalVariables|Getcohesion))) (.X (Math|Vector|BreakVector (LocalVariables|Getseparation))))))
      (Variables|Default|SetCurrentVel (+ (.Y (Math|Vector|BreakVector (Variables|Default|GetCurrentVel))) (+ (.Y (Math|Vector|BreakVector (LocalVariables|Getaligment))) (.Y (Math|Vector|BreakVector (LocalVariables|Getcohesion))) (.Y (Math|Vector|BreakVector (LocalVariables|Getseparation))))))
      (bind _output_get (Variables|Default|SetCurrentVel (+ (.Z (Math|Vector|BreakVector (Variables|Default|GetCurrentVel))) (+ (.Z (Math|Vector|BreakVector (LocalVariables|Getaligment))) (.Z (Math|Vector|BreakVector (LocalVariables|Getcohesion))) (.Z (Math|Vector|BreakVector (LocalVariables|Getseparation))))))))
    (:then_4
      (Variables|Default|SetCurrentVel (+ (.X (Math|Vector|BreakVector (Variables|Default|GetCurrentVel))) (+ (* (.X (Math|Vector|BreakVector (LocalVariables|Getaligment))) (LocalVariables|GetaligmentWeight)) (* (.X (Math|Vector|BreakVector (LocalVariables|Getcohesion))) (LocalVariables|GetcohesionWeight)) (* (.X (Math|Vector|BreakVector (LocalVariables|Getseparation))) (LocalVariables|GetseparationWeight)))))
      (Variables|Default|SetCurrentVel (+ (.Y (Math|Vector|BreakVector (Variables|Default|GetCurrentVel))) (+ (* (.Y (Math|Vector|BreakVector (LocalVariables|Getaligment))) (LocalVariables|GetaligmentWeight)) (* (.Y (Math|Vector|BreakVector (LocalVariables|Getcohesion))) (LocalVariables|GetcohesionWeight)) (* (.Y (Math|Vector|BreakVector (LocalVariables|Getseparation))) (LocalVariables|GetseparationWeight)))))
      (Variables|Default|SetCurrentVel (+ (.Z (Math|Vector|BreakVector (Variables|Default|GetCurrentVel))) (+ (* (.Z (Math|Vector|BreakVector (LocalVariables|Getaligment))) (LocalVariables|GetaligmentWeight)) (* (.Z (Math|Vector|BreakVector (LocalVariables|Getcohesion))) (LocalVariables|GetcohesionWeight)) (* (.Z (Math|Vector|BreakVector (LocalVariables|Getseparation))) (LocalVariables|GetseparationWeight))))))))